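; LightSwitchBox is a trigger actor that shows its attached lights while a LightMovableCube overlaps its LightSwitchCollider and hides them when one leaves.
; BeginPlay caches all attached actors as the lights, with no type filter.
; Overlap begin and end pass an exact class check in IsLightCube, then SwitchLights sets each attached actor's root component visibility without propagating to children.
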(event OnComponentEndOverlap(LightSwitchCollider)
  (params (OverlappedComponent :type Primitive%20Component%20Object%20Reference) (OtherActor :type Actor%20Object%20Reference) (OtherComp :type Primitive%20Component%20Object%20Reference) (OtherBodyIndex :type Integer))
  ;[1 1 1] Turn off lights when not overlapping
  (bind _returnvalue (CallFunction|IsLightCube OtherActor))
  (if _returnvalue
    (CallFunction|SwitchLights false)))

(event OnComponentBeginOverlap(LightSwitchCollider)
  (params (OverlappedComponent :type Primitive%20Component%20Object%20Reference) (OtherActor :type Actor%20Object%20Reference) (OtherComp :type Primitive%20Component%20Object%20Reference) (OtherBodyIndex :type Integer) (bFromSweep :type Boolean) (SweepResult :type Hit%20Result%20Structure%20%28by%20ref%29))
  ;[1 1 1] Call to function to qualify cube
  (bind _returnvalue (CallFunction|IsLightCube OtherActor))
  ;[1 1 1] Trigger lights function
  (if _returnvalue
    (CallFunction|SwitchLights true)))

(event EventBeginPlay
  ;[1 1 1] Select all attached lights
  (Variables|Default|SetAttachedLights (Actor|GetAttachedActors)))

(fn ConstructionScript)

(fn IsLightCube
  (params (Object :type Object%20Object%20Reference))
  ;[1 1 1] Is object a light cube
  (return (== "/Game/Blueprints/LightMovableCube.LightMovableCube_C" (Utilities|GetClass Object))))

(fn SwitchLights
  (params (bNewVisibility :type Boolean))
  ;[1 1 1] Turn on all attached light
  (bind _array_element (Utilities|Array|ForEachLoopwithBreak (Variables|Default|GetAttachedLights))
    (:LoopBody
      (Rendering|SetVisibility (Variables|/Script/Engine.Actor|GetRootComponent _array_element) bNewVisibility false))))