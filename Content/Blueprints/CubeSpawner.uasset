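; CubeSpawner is a Blueprint that populates the level with movable cubes and can reset them.
; On BeginPlay it finds every MovableSpawnPoint, spawns that point's ClassToSpawn at its location with zero rotation and unit scale, and stores each cube in MovableCubeArray.
; Despite its name, DespawnCubes destroys nothing: it moves each stored cube back to that cube's SpawnLocation.
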(event EventBeginPlay
  (CallFunction|SpawnAllCubes))

(fn ConstructionScript)

(fn SpawnAllCubes
  ;[1 1 1] Get all spawns and iterate through
  (bind _outactors (Actor|GetAllActorsOfClass "/Game/Blueprints/MovableSpawnPoint.MovableSpawnPoint_C"))
  (bind _output_get (Variables|Default|SetSpawnerArray _outactors))
  (for _array_element _output_get
    ;[1 1 1] Get Location and make transform
    (Variables|Default|SetLocation (Math|Transform|MakeTransform (Transformation|GetActorLocation _array_element)))
    ;[1 1 1] Instationate cube and add reference to array
    (bind _returnvalue (Game|SpawnActorfromClass (Variables|/Game/Blueprints/MovableSpawnPoint.MovableSpawnPoint_C|GetClassToSpawn _array_element) (Variables|Default|GetLocation) "Undefined" 0 0))
    (Utilities|Array|Add (Variables|Default|GetMovableCubeArray) _returnvalue)))

(fn DespawnCubes
  ;[1 1 1] For each spawned cube
  (for _array_element (Variables|Default|GetMovableCubeArray)
    (Transformation|SetActorLocationAndRotation _array_element (Variables|/Game/Blueprints/MovableCube.MovableCube_C|GetSpawnLocation _array_element))))