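; MovableCube is a physics cube that can be lifted with telekinesis and respawned at its starting location.
; Lifted and Drop swap linear damping and material and toggle the picked-up flag, with Drop also zeroing velocity.
; ShowCanLiftWidget briefly shows a prompt that a timer hides, while Tick keeps it offset from the mesh with camera-derived yaw.
; Respawn teleports the actor to the location stored at BeginPlay.
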(event Custom|Lifted
  ;[1 1 1] Reduce linear movement
  (Class|PrimitiveComponent|SetLinearDamping (Variables|Default|GetStaticMeshComponent0) (Variables|Default|GetliftingLinearDampening))
  ;[1 1 1] Set lifted material
  (Rendering|Material|SetMaterial (Variables|Default|GetStaticMeshComponent0) 0 "/Game/TelekonesisM.TelekonesisM")
  ;[1 1 1] switch picked up bool
  (Variables|Default|SetisPickedUp (not (Variables|Default|GetisPickedUp))))

(event Custom|UnshowWidget
  (Rendering|SetVisibility (Variables|Default|GetCanLiftWidget) false true))

(event Custom|Drop
  (Physics|SetPhysicsLinearVelocity (Variables|Default|GetStaticMeshComponent0) "0, 0, 0" false "None")
  ;[1 1 1] Set linear movement to normal
  (Class|PrimitiveComponent|SetLinearDamping (Variables|Default|GetStaticMeshComponent0) (Variables|Default|GetdefaultLinearDampening))
  ;[1 1 1] set none lifted material
  (Rendering|Material|SetMaterial (Variables|Default|GetStaticMeshComponent0) 0 (Variables|Default|GetDefaultMaterial))
  ;[1 1 1] Switch local picked up bool
  (Variables|Default|SetisPickedUp (not (Variables|Default|GetisPickedUp))))

(event Custom|ShowCanLiftWidget
  ;[1 1 1] Turn widget visible and set not visible .1s later
  (Rendering|SetVisibility (Variables|Default|GetCanLiftWidget) true true)
  (Utilities|Time|SetTimerbyEvent (delegate Custom|UnshowWidget) 0.1))

(event EventTick
  (params (DeltaSeconds :type Float%20%28single-precision%29))
  (CallFunction|ResolveWidgetPos))

(event EventRespawn
  ;[1 1 1] Call using interface
  (CallFunction|RespawnCube))

(event EventBeginPlay
  ;[1 1 1] Set widget text
  (Rendering|Components|TextRender|SetText (Variables|Default|GetCanLiftText) (Variables|Default|GetWidgetText))
  ;[1 1 1] Set widget to not visible
  (Rendering|SetVisibility (Variables|Default|GetCanLiftWidget) false true)
  ;[1 1 1] Store Spawn Postion
  (Variables|Default|SetSpawnLocation (Transformation|GetActorLocation))
  ;[1 1 1] set start Material as default
  (bind _asmaterial (Utilities|Casting|CastToMaterial (Rendering|Material|GetMaterial (Variables|Default|GetStaticMeshComponent0) 0)))
  (Variables|Default|SetDefaultMaterial _asmaterial)
  ;[1 1 1] Set default dampening
  (Class|PrimitiveComponent|SetLinearDamping (Variables|Default|GetStaticMeshComponent0) (Variables|Default|GetdefaultLinearDampening)))

(fn ConstructionScript)

(fn ResolveWidgetPos
  (bind _returnvalue (Game|GetPlayerCameraManager 0))
  (Transformation|SetWorldRotation (Variables|Default|GetCanLiftWidget) (Math|Rotator|MakeRotator 0.0 0.0 (+ (.Yaw (Math|Rotator|BreakRotator (Math|Rotator|FindLookatRotation (Transformation|GetWorldLocation (Variables|/Script/Engine.Actor|GetRootComponent _returnvalue)) (Camera|GetCameraLocation _returnvalue)))) 1.8e+02)) false false)
  (Transformation|SetWorldLocation (Variables|Default|GetCanLiftWidget) (+ (Transformation|GetWorldLocation (Variables|Default|GetStaticMeshComponent0)) "0.000000,-40.000000,90.000000") false false))

(fn RespawnCube
  (Transformation|SetActorLocation (Variables|Default|GetSpawnLocation) false false))