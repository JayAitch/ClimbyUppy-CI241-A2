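; JumpyCube is a cube actor that acts as a launch pad for the third-person character.
; When its LaunchPad volume is overlapped and the cube is not picked up, it casts the overlapping actor to ThirdPersonCharacter and launches it.
; The launch follows the mesh's up vector scaled by LaunchForce, so the cube's orientation sets the direction, and adds to existing velocity.
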(event OnComponentBeginOverlap(LaunchPad)
  (params (OverlappedComponent :type Primitive%20Component%20Object%20Reference) (OtherActor :type Actor%20Object%20Reference) (OtherComp :type Primitive%20Component%20Object%20Reference) (OtherBodyIndex :type Integer) (bFromSweep :type Boolean) (SweepResult :type Hit%20Result%20Structure%20%28by%20ref%29))
  ;[1 1 1] Collidingwith launch pad volume
  ;[1 1 1] If cube is not picked up
  (if (not (Variables|Default|GetisPickedUp))
    ;[1 1 1] Cast to TPC and launch
    (bind _asthird_person_character (Utilities|Casting|CastToThirdPersonCharacter OtherActor))
    (Character|LaunchCharacter _asthird_person_character (* (Math|Vector|GetUpVector (Variables|Default|GetStaticMeshComponent0)) (Variables|Default|GetLaunchForce)) false false)))

(event EventBeginPlay
  (|CallParentFunction) ; This node is disabled and will not be called.\nDrag off pins to build functionality.
)

(event EventTick
  (params (DeltaSeconds :type Float%20%28single-precision%29))
  (|CallParentFunction DeltaSeconds) ; This node is disabled and will not be called.\nDrag off pins to build functionality.
)

(fn ConstructionScript
  (|CallParentFunction))